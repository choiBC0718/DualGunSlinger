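; BP_GameMode is a Game Mode Blueprint that saves and loads score data through a save slot named for the best score.
; SaveScoreData writes the given value into a new BP_SaveGame object and overwrites the slot, without comparing it to the stored score.
; LoadScoreData checks that the slot exists, casts the loaded object to BP_SaveGame and returns its ScoreData.
; BeginPlay, Tick and the construction script are empty.
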(event `self.ReceiveBeginPlay`)

(fn `LoadScoreData`
  (returns (BestScore :type Integer))
  (bind _returnvalue (`GameplayStatics.DoesSaveGameExist` "BestScoreData"))
  (if _returnvalue
    (bind _returnvalue_2 (`GameplayStatics.LoadGameFromSlot` "BestScoreData"))
    (bind _asbp_save_game (cast `/Game/_WorkSpace/Blueprint/BP_SaveGame` _returnvalue_2))
    (return (`/Game/_WorkSpace/Blueprint/BP_SaveGame.ScoreData` _asbp_save_game))))

(fn `SaveScoreData`
  (params (SaveValue :type Integer))
  (bind _returnvalue (`GameplayStatics.CreateSaveGameObject` "/Game/_WorkSpace/Blueprint/BP_SaveGame.BP_SaveGame_C"))
  (bind _output_get (set `self.Save Instance` _returnvalue))
  (set `/Game/_WorkSpace/Blueprint/BP_SaveGame.ScoreData` SaveValue _output_get)
  (`GameplayStatics.SaveGameToSlot` _output_get "BestScoreData"))

(fn `UserConstructionScript`)